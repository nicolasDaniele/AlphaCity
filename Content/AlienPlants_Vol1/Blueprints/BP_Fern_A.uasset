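; BP_Fern_A is a physics-reactive fern that stands in for an instanced foliage fern near the player.
; Overlap by the player or a "Physics"-tagged actor simulates bodies below the trunk and plays a rustle.
; A polling loop detects the player leaving the MPC physics radius, blends physics weight by timeline, then re-adds the fern as a foliage instance and destroys the actor.
; Small ferns drop their blocking capsule; the glow animation is unconnected.
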(event OnComponentBeginOverlap(Capsule)
  (params (OverlappedComponent :type Primitive%20Component%20Object%20Reference) (OtherActor :type Actor%20Object%20Reference) (OtherComp :type Primitive%20Component%20Object%20Reference) (OtherBodyIndex :type Integer) (bFromSweep :type Boolean) (SweepResult :type Hit%20Result%20Structure%20%28by%20ref%29))
  ;[1 1 1] When Hit by Physics
  (if (or (== OtherActor (Game|Player|GetPlayerPawn 0)) (Actor|ActorHasTag OtherActor "Physics"))
    ;;[1 1 1] Simulate Physics
    (Class|SkeletalMeshComponent|SetAllBodiesBelowSimulatePhysics (Variables|Default|GetSK_Fern_A) (Utilities|String|StringToName "b_Trunk") true true)
    (Audio|PlaySoundatLocation "/Game/AlienPlants_Vol1/Sound/Foliage/SC_Foliage_Rustle.SC_Foliage_Rustle" (Transformation|GetWorldLocation (Variables|Default|GetCapsule)) "0, 0, 0" 1.0 1.0 0.0 0 0 0 0)))

(event EventBeginPlay
  (bind _sk_fern_a (Variables|Default|GetSK_Fern_A))
  ;[1 1 1] If the tree is large, keep the Capsule_Block to stop the player from pushing it over. Otherwise, delete the Capsule_Block
  (if (> (.SphereRadius (Collision|GetComponentBounds (Variables|Default|GetSK_Fern_A))) 2e+02)
    _
    (else
      (Components|DestroyComponent (Variables|Default|GetCapsule_Block))))
  (bind _returnvalue (Rendering|Material|GetScalarParameterValue "/Game/AlienPlants_Vol1/Materials/MaterialFunctions/MPC_FoliagePhysics.MPC_FoliagePhysics" "PhysicsRadius" :!class /Script/Engine.KismetMaterialLibrary))
  (Variables|Default|SetPhysicsRadius _returnvalue)
  ;[1 1 1] Get reference to Foliage World Actor
  (bind _outactors (Actor|GetAllActorsOfClass "/Script/Foliage.InstancedFoliageActor"))
  (Variables|Default|SetWorldFoliage (Utilities|Array|Get(acopy) _outactors))
  (Utilities|FlowControl|Delay 0.1 :!label _label)
  (if (> (Transformation|GetDistanceTo (Game|GetPlayerCharacter 0) self) (+ (Variables|Default|GetPhysicsRadius) 1e+02))
    (Utilities|FlowControl|DoOnce false
      (:Completed
        (bind _newtrack_0 (Timeline|Timeline_0 PlayFromStart)
          (:Update
            (bind _output_get (Variables|Default|SetPhysicsAlpha _newtrack_0))
            (Class|SkeletalMeshComponent|SetAllBodiesBelowPhysicsBlendWeight (Variables|Default|GetSK_Fern_A) (Utilities|String|StringToName "b_Base") _output_get false true))
          (:Finished
            (Collision|SetCollisionEnabled _sk_fern_a "NoCollision")
            (Physics|SetSimulatePhysics _sk_fern_a false)
            (for (_array_element _array_index) (Actor|GetComponentsByClass (Variables|Default|GetWorldFoliage) "/Script/Engine.InstancedStaticMeshComponent")
              (if (Utilities|String|Contains (Utilities|GetDisplayName _array_element) "Fern_A")
                (Variables|Default|SetClassIndex _array_index)))
            (Utilities|FlowControl|DoOnce false
              (:Completed
                (Components|InstancedStaticMesh|AddInstance (Utilities|Array|Get(acopy) (Actor|GetComponentsByClass (Variables|Default|GetWorldFoliage) "/Script/Engine.InstancedStaticMeshComponent") (Variables|Default|GetClassIndex)) (Transformation|GetWorldTransform (Variables|Default|GetSK_Fern_A)) false)
                (Actor|DestroyActor)))))))
    (else
      (goto _label))))

(fn ConstructionScript
  (bind _sk_fern_a (Variables|Default|GetSK_Fern_A))
  (bind _returnvalue (Rendering|Material|CreateDynamicMaterialInstance (Rendering|Material|GetMaterial _sk_fern_a 0) "None" "None" :!class /Script/Engine.KismetMaterialLibrary))
  (bind _output_get (Variables|Default|SetMaterial _returnvalue))
  (Rendering|Material|SetMaterial _sk_fern_a 0 _output_get)
  (bind _returnvalue_2 (Rendering|Material|GetScalarParameterValue _output_get "Glow_Min_Amount" :!class /Script/Engine.MaterialInstanceDynamic))
  (Variables|Default|SetDefault_GlowAmount _returnvalue_2))