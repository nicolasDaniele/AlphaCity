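; Player controller that hosts the Ready Player Me avatar creator UI, toggled loader via Q, and a hidden traveling loader widget.
; Preview avatars spawn through the game mode on authority, then a server-to-client event chain hands the actor to the editor panel's renderer.
; Loading an avatar URL from the UI updates the AlphaCharacter, whose update-state events drive the creator's throbber.
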(event Custom|OnAvatarUpdatedEvent
  (params (IsUpdating :type Boolean))
  (bind _avatarcreatorwrapperwidget (Variables|Default|GetAvatarCreatorWrapperWidget)
    (:then
      (Default|SetThrobberVisibility _avatarcreatorwrapperwidget IsUpdating))
    (:else)))

(event Custom|OnLoadAvatar
  (params (Url :type String))
  ;[1 1 1 1 30] UI Callbacks for Avatar Saved
  (bind _alphacharacter (Variables|Default|GetAlphaCharacter)
    (:then
      (Default|UpdateAvatar _alphacharacter Url)
      (bind _avatarcreatorwrapperwidget (Variables|Default|GetAvatarCreatorWrapperWidget)
        (:then
          (Default|SetThrobberVisibility _avatarcreatorwrapperwidget true))
        (:else)))
    (:else)))

(event Custom|Server_SetupPreviewAvatar
  (bind _returnvalue (Game|GetGameMode))
  (bind _asbp_alpha_game_mode (Utilities|Casting|CastToBP_AlphaGameMode _returnvalue))
  (bind _spawnedpreviewactor (Default|GetPreviewActor _asbp_alpha_game_mode))
  (Utilities|IsValid _spawnedpreviewactor
    (:Is%20Valid
      (CallFunction|ClientSetupPreviewAvatar _spawnedpreviewactor))))

(event Custom|CreatePreviewAvatar
  (params (AvatarClass :type Actor%20Class%20Reference))
  (Networking|SwitchHasAuthority
    (:Authority
      (Default|TrySpawningPreviewAvatar (.AsBP%20Alpha%20Game%20Mode (Utilities|Casting|CastToBP_AlphaGameMode (Game|GetGameMode))) AvatarClass))
    (:Remote
      _))
  (CallFunction|ServerSetupPreviewAvatar))

(event Custom|Client_SetupPreviewAvatar
  (params (Avatar :type Actor%20Object%20Reference))
  (Utilities|IsValid Avatar
    (:Is%20Valid
      (bind _avatarcreatorwrapperwidget (Variables|Default|GetAvatarCreatorWrapperWidget)
        (:then
          (Variables|/ReadyPlayerMe/ReadyPlayerMe/AvatarCreator/Widgets/Editor/WBP_RPM_Renderer.WBP_RPM_Renderer_C|SetRendererActor (Variables|/ReadyPlayerMe/ReadyPlayerMe/AvatarCreator/Widgets/Editor/WBP_RPM_AvatarEditor.WBP_RPM_AvatarEditor_C|GetAvatarRenderer (Variables|/ReadyPlayerMe/ReadyPlayerMe/AvatarCreator/Widgets/WBP_RPM_AvatarCreator.WBP_RPM_AvatarCreator_C|GetAvatarEditorPanel (Variables|/ReadyPlayerMe/ReadyPlayerMe/QuickStart/Widgets/WBP_RPM_AvatarCreatorWrapper.WBP_RPM_AvatarCreatorWrapper_C|GetAvatarCreator _avatarcreatorwrapperwidget))) Avatar)
          (if (Utilities|DoesObjectImplementInterface Avatar "/ReadyPlayerMe/ReadyPlayerMe/AvatarCreator/Blueprints/BI_RPM_PreviewAvatar.BI_RPM_PreviewAvatar_C")
            (bind _asbi_rpm_preview_avatar (Utilities|Casting|CastToBI_RPM_PreviewAvatar Avatar))
            (Variables|/ReadyPlayerMe/ReadyPlayerMe/AvatarCreator/Widgets/Editor/WBP_RPM_Renderer.WBP_RPM_Renderer_C|SetPreviewAvatar (Variables|/ReadyPlayerMe/ReadyPlayerMe/AvatarCreator/Widgets/Editor/WBP_RPM_AvatarEditor.WBP_RPM_AvatarEditor_C|GetAvatarRenderer (Variables|/ReadyPlayerMe/ReadyPlayerMe/AvatarCreator/Widgets/WBP_RPM_AvatarCreator.WBP_RPM_AvatarCreator_C|GetAvatarEditorPanel (Variables|/ReadyPlayerMe/ReadyPlayerMe/QuickStart/Widgets/WBP_RPM_AvatarCreatorWrapper.WBP_RPM_AvatarCreatorWrapper_C|GetAvatarCreator _avatarcreatorwrapperwidget))) _asbi_rpm_preview_avatar)
            (Default|ApplyCustomProperties (Variables|/ReadyPlayerMe/ReadyPlayerMe/AvatarCreator/Widgets/Editor/WBP_RPM_AvatarEditor.WBP_RPM_AvatarEditor_C|GetAvatarRenderer (Variables|/ReadyPlayerMe/ReadyPlayerMe/AvatarCreator/Widgets/WBP_RPM_AvatarCreator.WBP_RPM_AvatarCreator_C|GetAvatarEditorPanel (Variables|/ReadyPlayerMe/ReadyPlayerMe/QuickStart/Widgets/WBP_RPM_AvatarCreatorWrapper.WBP_RPM_AvatarCreatorWrapper_C|GetAvatarCreator _avatarcreatorwrapperwidget))))))
        (:else)))))

(event EventBeginPlay
  (Utilities|FlowControl|Sequence
    (:then_0
      (if (Pawn|IsLocalPlayerController)
        ;[1 1 1 1 31] UI Creation
        (Utilities|IsValid (Variables|Default|GetAvatarCreatorWrapperWidget)
          (:Is%20Not%20Valid
            (bind _returnvalue (UserInterface|CreateWidget "/ReadyPlayerMe/ReadyPlayerMe/QuickStart/Widgets/WBP_RPM_AvatarCreatorWrapper.WBP_RPM_AvatarCreatorWrapper_C"))
            (bind _output_get (Variables|Default|SetAvatarCreatorWrapperWidget _returnvalue))
            (Utilities|IsValid _output_get
              (:Is%20Valid
                (UserInterface|Viewport|AddtoViewport _output_get 0)))))))
    (:then_1
      (bind _asbp_alpha_character (Utilities|Casting|CastToBP_AlphaCharacter (Game|Player|GetPlayerPawn 0)))
      (bind _output_get_2 (Variables|Default|SetAlphaCharacter _asbp_alpha_character))
      (Utilities|IsValid _output_get_2
        (:Is%20Valid
          (EventDispatchers|BindEventtoOnAvatarUpdateStateChanged _output_get_2 (delegate Custom|OnAvatarUpdatedEvent)))))
    (:then_2
      ;[1 1 1 1 30] UI Callbacks for Avatar Saved
      (bind _avatarcreatorwrapperwidget (Variables|Default|GetAvatarCreatorWrapperWidget)
        (:then
          (EventDispatchers|BindEventtoOnLoadAvatar _avatarcreatorwrapperwidget (delegate Custom|OnLoadAvatar)))
        (:else)))
    (:then_3
      ;[1 1 1 1 26] Traveling Loader Creation & Binding
      (bind _returnvalue_2 (UserInterface|CreateWidget "/Game/UI/WBP_TravelingLoader.WBP_TravelingLoader_C"))
      (bind _output_get_3 (Variables|Default|SetTravelingLoader _returnvalue_2))
      (Utilities|IsValid _output_get_3
        (:Is%20Valid
          (Variables|/Script/UMG.Widget|SetVisibility _output_get_3 "Hidden")
          (UserInterface|Viewport|AddtoViewport _output_get_3 0))))))

(event Input|KeyboardEvents|Q
  (params (Key :type Key%20Structure :default "None"))
  ;[1 1 1] Show/Hide RPM Loader Widget on Key press
  (:Pressed
    (bind _avatarcreatorwrapperwidget (Variables|Default|GetAvatarCreatorWrapperWidget)
      (:then
        (Default|ToggleLoaderVisibility _avatarcreatorwrapperwidget))
      (:else))))

(fn ConstructionScript)