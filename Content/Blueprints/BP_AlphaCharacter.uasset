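; Player character with a Ready Player Me avatar, level travel and momentum-preserving teleport.
; BeginPlay sets game-only input and reloads the AvatarSubsystem's saved URL through a Server-to-Client event chain; completed loads write the URL back and refresh the animation class by body type.
; Teleport offsets the destination, aligns control rotation and redirects speed along the new forward vector.
; Travel events forward level names to AlphaPlayerController via player index 0.
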(event Custom|Server_TryTravel
  (params (LevelName :type String))
  (CallFunction|ClientTryTrvel LevelName))

(event Custom|Client_TryTrvel
  (params (LevelName :type String))
  (bind _asalpha_player_controller (Utilities|Casting|CastToAlphaPlayerController (Game|GetPlayerController 0)))
  (Class|AlphaPlayerController|TryTraveltoLevel _asalpha_player_controller LevelName))

(event Custom|Client_SaveAvatar
  (params (TargetRPMComp :type Ready%20Player%20Me%20Component%20Object%20Reference) (Url :type String))
  ;[0 0 0] RPM Save and Update Avatar
  (Class|ReadyPlayerMeComponent|LoadNewAvatar TargetRPMComp Url (delegate Custom|OnAvatarLoadComplete) (delegate Custom|On%20Load%20Failed)))

(event Custom|OnAvatarLoadComplete
  ;[0 0 0] RPM Save and Update Avatar
  (CallFunction|UpdateAnimator)
  (Class|AvatarSubsystem|UpdateMeshUrl (Subsystems|GetAvatarSubsystem) (Variables|/Script/ReadyPlayerMe.ReadyPlayerMeComponent|GetUrlShortcode (Variables|Default|GetReadyPlayerMe)))
  (Default|CallOnAvatarUpdateStateChanged false))

(event Custom|Server_SaveAvatar
  (params (Target :type Ready%20Player%20Me%20Component%20Object%20Reference) (Url :type String))
  ;[0 0 0] RPM Save and Update Avatar
  (CallFunction|ClientSaveAvatar Target Url))

(event Custom|On%20Load%20Failed
  (params (ErrorMessage :type String))
  ;[0 0 0] RPM Save and Update Avatar
  (Development|PrintString ErrorMessage true true "(R=0.000000,G=0.660000,B=1.000000,A=1.000000)" 5.0)
  (CallFunction|UpdateAnimator))

(event Custom|UpdateAnimator
  (bind _mesh (Variables|Character|GetMesh))
  (bind _readyplayerme (Variables|Default|GetReadyPlayerMe))
  (bind _avatarmetadata (Variables|/Script/ReadyPlayerMe.ReadyPlayerMeComponent|GetAvatarMetadata _readyplayerme))
  (bind _bodytype (Utilities|Struct|BreakAvatarMetadata _avatarmetadata))
  ;[0 0 0] Update animations
  (switch Utilities|FlowControl|Switch|SwitchonEAvatarBodyType _bodytype
    (:Undefined
      (Class|SkeletalMeshComponent|SetAnimClass _mesh))
    (:FullBody
      (Development|PrintString (Utilities|String|Append "Animations do not exist for the bodytype: " (Utilities|String|EnumtoString _bodytype)) :!label _label)
      (Class|SkeletalMeshComponent|SetAnimClass _mesh "/ReadyPlayerMe/ReadyPlayerMe/QuickStart/Animations/ABP_RPM_ThirdPerson.ABP_RPM_ThirdPerson_C"))
    (:HalfBody
      (goto _label))))

(event Custom|UpdateAvatar
  (params (Url :type String))
  ;[0 0 0] RPM Save and Update Avatar
  (CallFunction|ServerSaveAvatar (Variables|Default|GetReadyPlayerMe) Url))

(event EventDestroyed)

(event EventBlueprintTestFunction
  (params (LevelToTravel :type String))
  (CallFunction|ClientTryTrvel LevelToTravel))

(event EventBeginPlay
  (bind _returnvalue (Game|GetPlayerController 0))
  (bind _returnvalue_2 (Subsystems|GetAvatarSubsystem))
  (bind _returnvalue_3 (Class|AvatarSubsystem|GetCurrentMeshUrl _returnvalue_2))
  (Utilities|FlowControl|Sequence
    (:then_0
      (Variables|/Script/Engine.PlayerController|SetbShowMouseCursor _returnvalue false)
      (Input|SetInputModeGameOnly _returnvalue false))
    (:then_1
      (Utilities|IsValid _returnvalue_2
        (:Is%20Valid
          (if (not (Utilities|Array|IsEmpty _returnvalue_3))
            (CallFunction|UpdateAvatar _returnvalue_3)
            (Default|CallOnAvatarUpdateStateChanged true)))))
    (:then_2
      (Variables|Default|SetLinear%20Color (Utilities|Struct|MakeLinearColor (Math|Random|RandomFloatinRange 0.0 1.0) (Math|Random|RandomFloatinRange 0.0 1.0) (Math|Random|RandomFloatinRange 0.0 1.0) 1.0)))))

(event EventTeleport
  (params (targetLocation :type Vector :default "0, 0, 0") (targetDirection :type Vector :default "0, 0, 0") (targetRotation :type Rotator :default "0, 0, 0"))
  (Variables|Default|SetVelocityMagnitude (Math|Vector|VectorLength (Transformation|GetVelocity)))
  (Transformation|SetActorLocationAndRotation (+ targetLocation (* targetDirection 4e+01)) targetRotation)
  (Pawn|SetControlRotation (Pawn|GetController) targetRotation)
  (Variables|/Script/Engine.MovementComponent|SetVelocity (Variables|Character|GetCharacterMovement) (* (Transformation|GetActorForwardVector) (Variables|Default|GetVelocityMagnitude))))

(fn ConstructionScript)