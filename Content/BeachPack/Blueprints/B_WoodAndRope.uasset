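; Editor-built wood pole and rope fence that the construction script lays along a spline, with no active runtime logic.
; It places instanced poles at fixed spacing, stretches scaled rope instances between their tops, and starts new instanced components every ten poles.
; NoRope flags cut gaps, dropping poles between two empty segments.
; A self-resetting toggle traces down to snap spline points and the actor to the ground.
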(event EventBeginPlay)

(event Collision|EventActorBeginOverlap
  (params (OtherActor :type Actor%20Object%20Reference)))

(event EventTick
  (params (DeltaSeconds :type Float%20%28single-precision%29)))

(fn ConstructionScript
  (bind _spline (Variables|Default|GetSpline))
  (bind _distancepoles (Variables|General|GetDistancePoles))
  (bind _norope (Variables|General|GetNoRope))
  (bind _spline_2 (Variables|Default|GetSpline))
  (bind _spline_3 (Variables|Default|GetSpline))
  (bind _defaultsceneroot (Variables|Default|GetDefaultSceneRoot))
  (bind _defaultsceneroot_2 (Variables|Default|GetDefaultSceneRoot))
  (bind _spline_4 (Variables|Default|GetSpline))
  (bind _spline_5 (Variables|Default|GetSpline))
  (bind _returnvalue (Spline|GetSplineLength _spline_5))
  (bind _returnvalue_2 (Spline|GetLocationatSplinePoint _spline_3 0 "World"))
  (bind _returnvalue_3 (Transformation|GetWorldLocation _defaultsceneroot_2))
  (bind (_x _y _z) (Math|Vector|BreakVector _returnvalue_3))
  (bind _returnvalue_4 (/ _returnvalue _distancepoles))
  (bind _returnvalue_5 (Math|Float|Truncate _returnvalue_4))
  (bind _returnvalue_6 (+ _returnvalue_5 1))
  ;[0.6875 0 1] SnappingSplineToGround
  (if (Variables|Snap|GetSnappingSplineToTheGround)
    (for _index (range 0 (- (Spline|GetNumberOfSplinePoints (Variables|Default|GetSpline)) 1))
      (bind (_outhit _returnvalue_7) (Collision|LineTraceByChannel (Spline|GetLocationatSplinePoint (Variables|Default|GetSpline) _index "World") (+ (Spline|GetLocationatSplinePoint (Variables|Default|GetSpline) _index "World") "0.000000,-0.000000,-10000.000000") "TraceTypeQuery1" false 0 "None"))
      (if _returnvalue_7
        (Variables|Snap|SetLocationPoint (+ (Math|Transform|InverseTransformLocation (Math|Transform|MakeTransform (Transformation|GetWorldLocation _defaultsceneroot) (Variables|/Script/Engine.SceneComponent|GetRelativeRotation _defaultsceneroot) (Variables|/Script/Engine.SceneComponent|GetRelativeScale3D _defaultsceneroot)) (.Location (Collision|BreakHitResult _outhit))) "0, 0,2.000000"))
        (else
          (Variables|Snap|SetLocationPoint (Math|Vector|MakeVector (.X (Math|Vector|BreakVector (Spline|GetLocationatSplinePoint (Variables|Default|GetSpline) _index "Local"))) (.Y (Math|Vector|BreakVector (Spline|GetLocationatSplinePoint (Variables|Default|GetSpline) _index "Local"))) 0.0))))
      (Spline|SetLocationatSplinePoint (Variables|Default|GetSpline) _index (Variables|Snap|GetLocationPoint) "Local" true))
    (Variables|Snap|SetSnappingSplineToTheGround false)
    (Variables|Snap|SetZdifference (.Z (Math|Vector|BreakVector (- (Transformation|GetWorldLocation (Variables|Default|GetDefaultSceneRoot)) (Spline|GetLocationatSplinePoint (Variables|Default|GetSpline) 0 "World")))))
    (for _index_2 (range 0 (- (Spline|GetNumberOfSplinePoints (Variables|Default|GetSpline)) 1))
      (Spline|SetLocationatSplinePoint _spline_2 _index_2 (+ (Spline|GetLocationatSplinePoint _spline_2 _index_2 "Local") (Math|Vector|MakeVector 0.0 0.0 (Variables|Snap|GetZdifference))) "Local" true))
    (bind _outhit_2 (Collision|LineTraceByChannel _returnvalue_2 (+ _returnvalue_2 "0.000000,-0.000000,-10000.000000") "TraceTypeQuery1" false 0 "None"))
    (Transformation|SetWorldLocation (Variables|Default|GetDefaultSceneRoot) (+ (Math|Vector|MakeVector _x _y (- _z (- (- (.Z (Math|Vector|BreakVector _returnvalue_2)) (Variables|Snap|GetSnapOffset)) (.Z (Math|Vector|BreakVector (.Location (Collision|BreakHitResult _outhit_2))))))) "0, 0,5.000000") false false))
  (Variables|General|SetCurrentLength 0.0)
  (Utilities|Array|Resize (Variables|General|GetNoRope) _returnvalue_6)
  (for _index_3 (range 0 _returnvalue_6)
    (if (== (Math|Integer|%(Integer) _index_3 10) 0)
      (bind _returnvalue_8 (AddComponent|AddInstancedStaticMeshComponent false))
      (if (== (Variables|General|GetPole%20Type) 1)
        (Components|StaticMesh|SetStaticMesh _returnvalue_8 "/Game/BeachPack/Models/SM_PoleWood_02.SM_PoleWood_02")
        (else
          (Components|StaticMesh|SetStaticMesh _returnvalue_8 "/Game/BeachPack/Models/SM_PoleWood_01.SM_PoleWood_01")))
      (Variables|Default|SetInstancesPole _returnvalue_8)
      (bind _returnvalue_9 (AddComponent|AddInstancedStaticMeshComponent false))
      (Variables|Default|SetInstancesRope _returnvalue_9))
    (if (and (Utilities|Array|Get(acopy) _norope (Math|Integer|Clamp(Integer) _index_3 0 (- (Utilities|Array|Length (Variables|General|GetNoRope)) 1))) (Utilities|Array|Get(acopy) _norope (Math|Integer|Clamp(Integer) (- _index_3 1) 0 100000)))
      _
      (else
        (Components|InstancedStaticMesh|AddInstance (Variables|Default|GetInstancesPole) (Math|Transform|MakeTransform (Spline|GetLocationatDistanceAlongSpline _spline_4 (Variables|General|GetCurrentLength) "Local") (Spline|GetRotationatDistanceAlongSpline _spline_4 (Variables|General|GetCurrentLength) "Local")) false)))
    (if (not (== _index_3 (+ (Math|Float|Truncate (/ (Spline|GetSplineLength (Variables|Default|GetSpline)) (Variables|General|GetDistancePoles))) 1)))
      (if (Utilities|Array|Get(acopy) (Variables|General|GetNoRope) _index_3)
        _
        (else
          (Components|InstancedStaticMesh|AddInstance (Variables|Default|GetInstancesRope) (Math|Transform|MakeTransform (+ (Spline|GetLocationatDistanceAlongSpline _spline (Variables|General|GetCurrentLength) "Local") (* (Class|SplineComponent|GetUpVectoratDistanceAlongSpline _spline (Variables|General|GetCurrentLength) "Local") "92.000000,92.000000,92.000000")) (Math|Rotator|MakeRotator (.Roll (Math|Rotator|BreakRotator (Math|Rotator|FindLookatRotation (+ (Spline|GetLocationatDistanceAlongSpline _spline (Variables|General|GetCurrentLength) "Local") (* (Class|SplineComponent|GetUpVectoratDistanceAlongSpline _spline (Variables|General|GetCurrentLength) "Local") "92.000000,92.000000,92.000000")) (+ (Spline|GetLocationatDistanceAlongSpline _spline (+ (Variables|General|GetCurrentLength) (Variables|General|GetDistancePoles)) "Local") (* (Class|SplineComponent|GetUpVectoratDistanceAlongSpline _spline (+ (Variables|General|GetCurrentLength) (Variables|General|GetDistancePoles)) "Local") "92.000000,92.000000,92.000000"))))) (.Pitch (Math|Rotator|BreakRotator (Math|Rotator|FindLookatRotation (+ (Spline|GetLocationatDistanceAlongSpline _spline (Variables|General|GetCurrentLength) "Local") (* (Class|SplineComponent|GetUpVectoratDistanceAlongSpline _spline (Variables|General|GetCurrentLength) "Local") "92.000000,92.000000,92.000000")) (+ (Spline|GetLocationatDistanceAlongSpline _spline (+ (Variables|General|GetCurrentLength) (Variables|General|GetDistancePoles)) "Local") (* (Class|SplineComponent|GetUpVectoratDistanceAlongSpline _spline (+ (Variables|General|GetCurrentLength) (Variables|General|GetDistancePoles)) "Local") "92.000000,92.000000,92.000000"))))) (.Yaw (Math|Rotator|BreakRotator (Math|Rotator|FindLookatRotation (+ (Spline|GetLocationatDistanceAlongSpline _spline (Variables|General|GetCurrentLength) "Local") (* (Class|SplineComponent|GetUpVectoratDistanceAlongSpline _spline (Variables|General|GetCurrentLength) "Local") "92.000000,92.000000,92.000000")) (+ (Spline|GetLocationatDistanceAlongSpline _spline (+ (Variables|General|GetCurrentLength) (Variables|General|GetDistancePoles)) "Local") (* (Class|SplineComponent|GetUpVectoratDistanceAlongSpline _spline (+ (Variables|General|GetCurrentLength) (Variables|General|GetDistancePoles)) "Local") "92.000000,92.000000,92.000000")))))) (Math|Vector|MakeVector (/ (Math|Vector|Distance(Vector) (+ (Spline|GetLocationatDistanceAlongSpline _spline (Variables|General|GetCurrentLength) "Local") (* (Class|SplineComponent|GetUpVectoratDistanceAlongSpline _spline (Variables|General|GetCurrentLength) "Local") "92.000000,92.000000,92.000000")) (+ (Spline|GetLocationatDistanceAlongSpline _spline (+ (Variables|General|GetCurrentLength) (Variables|General|GetDistancePoles)) "Local") (* (Class|SplineComponent|GetUpVectoratDistanceAlongSpline _spline (+ (Variables|General|GetCurrentLength) (Variables|General|GetDistancePoles)) "Local") "92.000000,92.000000,92.000000"))) 2.5e+02) (/ (Math|Vector|Distance(Vector) (+ (Spline|GetLocationatDistanceAlongSpline _spline (Variables|General|GetCurrentLength) "Local") (* (Class|SplineComponent|GetUpVectoratDistanceAlongSpline _spline (Variables|General|GetCurrentLength) "Local") "92.000000,92.000000,92.000000")) (+ (Spline|GetLocationatDistanceAlongSpline _spline (+ (Variables|General|GetCurrentLength) (Variables|General|GetDistancePoles)) "Local") (* (Class|SplineComponent|GetUpVectoratDistanceAlongSpline _spline (+ (Variables|General|GetCurrentLength) (Variables|General|GetDistancePoles)) "Local") "92.000000,92.000000,92.000000"))) 2.5e+02) (/ (Math|Vector|Distance(Vector) (+ (Spline|GetLocationatDistanceAlongSpline _spline (Variables|General|GetCurrentLength) "Local") (* (Class|SplineComponent|GetUpVectoratDistanceAlongSpline _spline (Variables|General|GetCurrentLength) "Local") "92.000000,92.000000,92.000000")) (+ (Spline|GetLocationatDistanceAlongSpline _spline (+ (Variables|General|GetCurrentLength) (Variables|General|GetDistancePoles)) "Local") (* (Class|SplineComponent|GetUpVectoratDistanceAlongSpline _spline (+ (Variables|General|GetCurrentLength) (Variables|General|GetDistancePoles)) "Local") "92.000000,92.000000,92.000000"))) 2.5e+02))) false)))
      (Variables|General|SetCurrentLength (+ (Variables|General|GetCurrentLength) (Variables|General|GetDistancePoles))))))