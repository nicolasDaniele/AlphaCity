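; Wind randomizer actor that periodically varies a WindDirectionalSource's direction and speed for changing weather.
; The construction script grabs the first such source in the level if none is assigned.
; Tick feeds a Delay of randomized length around ChangeTimeS, so each expiry sets random roll and pitch, drifts yaw, and nudges speed within clamped limits.
; Changes apply instantly, without interpolation.
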(event EventBeginPlay)

(event Collision|EventActorBeginOverlap
  (params (OtherActor :type Actor%20Object%20Reference)))

(event EventTick
  (params (DeltaSeconds :type Float%20%28single-precision%29))
  (bind _returnvalue (Math|Random|RandomFloatinRange -2e+01 2.0))
  (bind _winddirection (Variables|Default|GetWindDirection))
  (bind _variation_speed (Variables|Default|GetVariation%20Speed))
  (bind _variation_rotation___z (Variables|Default|GetVariation%20Rotation%20-+Z))
  (bind _change_time__s_ (Variables|Default|GetChange%20Time%20%28s%29))
  (bind _winddirection_2 (Variables|Default|GetWindDirection))
  (bind _min_speed (Variables|Default|GetMin%20Speed))
  (bind _returnvalue_2 (/ _change_time__s_ 4))
  (bind _component (Variables|/Script/Engine.WindDirectionalSource|GetComponent _winddirection))
  (bind _component_2 (Variables|/Script/Engine.WindDirectionalSource|GetComponent _winddirection_2))
  ;[0.3125 0 1] Time to change
  (Utilities|FlowControl|Delay (Math|Conversions|ToFloat(Integer) (+ _change_time__s_ (Math|Random|RandomIntegerinRange (* _returnvalue_2 -1) _returnvalue_2))))
  ;[0 1 0.08594] Rotation
  (Transformation|SetRelativeRotation _component_2 (Math|Rotator|MakeRotator _returnvalue _returnvalue (+ (.yaw (Variables|/Script/Engine.SceneComponent|GetRelativeRotation _component_2)) (Math|Random|RandomFloatinRange (* _variation_rotation___z -1.0) (Math|Conversions|ToFloat(Integer) _variation_rotation___z)))) false false)
  ;[1 0.04688 0] Speed
  (Class|WindDirectionalSourceComponent|SetSpeed _component (Math|Float|Clamp(Float) (+ (Variables|/Script/Engine.WindDirectionalSourceComponent|GetSpeed _component) (Math|Random|RandomFloatinRange (* _variation_speed -1.0) _variation_speed)) _min_speed (Math|Float|Clamp(Float) (Variables|Default|GetMax%20Speed) _min_speed 1e+02))))

(fn ConstructionScript
  (Utilities|IsValid (Variables|Default|GetWindDirection)
    (:Is%20Not%20Valid
      (bind _outactors (Actor|GetAllActorsOfClass "/Script/Engine.WindDirectionalSource"))
      (Variables|Default|SetWindDirection (Utilities|Array|Get(acopy) _outactors)))))