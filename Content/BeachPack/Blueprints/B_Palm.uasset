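; Configurable palm tree actor for beach scenes, assembled entirely in the construction script with no runtime logic.
; Ticking Randomize acts as a one-shot button, rerolling each enabled option (trunk, materials, coconuts, scales) before resetting itself so the result persists.
; The chosen trunk mesh and material are applied, then leaves and optional coconuts are added as scaled mesh components on the trunk's sockets.
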(event EventBeginPlay)

(event Collision|EventActorBeginOverlap
  (params (OtherActor :type Actor%20Object%20Reference)))

(event EventTick
  (params (DeltaSeconds :type Float%20%28single-precision%29)))

(fn ConstructionScript
  (bind _rand_scale_min (Variables|Random|GetRand%20Scale%20Min))
  (bind _rand_scale_max (Variables|Random|GetRand%20Scale%20Max))
  (bind _returnvalue (Math|Random|RandomFloatinRange _rand_scale_min _rand_scale_max))
  (if (Variables|Random|GetRandomize)
    (if (Variables|Random|GetRand%20Trunk%20Type)
      (Variables|General|SetTrunkType (Math|Random|RandomIntegerinRange 1 (Utilities|Array|Length (Variables|Default|GetTrunkArray)))))
    (if (Variables|Random|GetRand%20Trunk%20Material)
      (Variables|General|SetTrunkMaterial (Math|Random|RandomIntegerinRange 1 (Utilities|Array|Length (Variables|Default|GetTrunkMaterialArray)))))
    (if (Variables|Random|GetRand%20Coconuts)
      (Variables|General|SetCoconuts (Math|Random|RandomBool)))
    (if (Variables|Random|GetRand%20Scale%20Leaves)
      (Variables|General|SetScaleLeaves (Math|Random|RandomFloatinRange 0.8 1.2)))
    (if (Variables|Random|GetRand%20Scale%20Coconuts)
      (Variables|General|SetScaleCoconuts (Math|Random|RandomFloatinRange 0.8 1.2)))
    (if (Variables|Random|GetRand%20Scale)
      (Transformation|SetRelativeScale3D (Variables|Default|GetDefaultSceneRoot) (Math|Vector|MakeVector _returnvalue _returnvalue _returnvalue)))
    (if (Variables|Random|GetRand%20Leaves%20Materials)
      (Variables|General|SetLeavesMaterial (Math|Random|RandomIntegerinRange 1 4)))
    (Variables|Random|SetRandomize false))
  (Components|StaticMesh|SetStaticMesh (Variables|Default|GetTrunk) (Utilities|Array|Get(acopy) (Variables|Default|GetTrunkArray) (- (Variables|General|GetTrunkType) 1)))
  (Rendering|Material|SetMaterial (Variables|Default|GetTrunk) 0 (Utilities|Array|Get(acopy) (Variables|Default|GetTrunkMaterialArray) (- (Variables|General|GetTrunkMaterial) 1)))
  (bind _returnvalue_2 (AddComponent|AddStaticMeshComponent false))
  (Transformation|AttachComponentToComponent _returnvalue_2 (Variables|Default|GetTrunk) "Leaves" "KeepRelative" "KeepRelative" "KeepRelative" true)
  (Transformation|SetRelativeScale3D _returnvalue_2 (Math|Vector|MakeVector (Variables|General|GetScaleLeaves) (Variables|General|GetScaleLeaves) (Variables|General|GetScaleLeaves)))
  (Rendering|Material|SetMaterial _returnvalue_2 0 (Utilities|Array|Get(acopy) (Variables|Default|GetLeavesMaterialArray) (- (Variables|General|GetLeavesMaterial) 1)))
  (if (Variables|General|GetCoconuts)
    (bind _returnvalue_3 (AddComponent|AddStaticMeshComponent false))
    (Transformation|AttachComponentToComponent _returnvalue_3 (Variables|Default|GetTrunk) "Coconuts" "KeepRelative" "KeepRelative" "KeepRelative" true)
    (Transformation|SetRelativeScale3D _returnvalue_3 (Math|Vector|MakeVector (Variables|General|GetScaleCoconuts) (Variables|General|GetScaleCoconuts) (Variables|General|GetScaleCoconuts)))))