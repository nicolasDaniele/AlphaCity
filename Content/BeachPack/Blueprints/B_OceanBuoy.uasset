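; B_OceanBuoy is an ocean buoy prop whose static mesh simulates physics.
; The construction script clamps a 1-based Material index to the Materials array, applies that material to the mesh, and sets angular and linear damping.
; BeginPlay enables physics simulation and reapplies both damping values.
; The graphs contain no buoyancy logic.
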(event EventBeginPlay
  (bind _staticmesh (Variables|Default|GetStaticMesh))
  (Physics|SetSimulatePhysics _staticmesh true)
  (Class|PrimitiveComponent|SetAngularDamping _staticmesh (Variables|General|GetAngular%20Damping))
  (Class|PrimitiveComponent|SetLinearDamping _staticmesh (Variables|General|GetLinear%20Damping)))

(event Collision|EventActorBeginOverlap
  (params (OtherActor :type Actor%20Object%20Reference)))

(event EventTick
  (params (DeltaSeconds :type Float%20%28single-precision%29)))

(fn ConstructionScript
  (bind _staticmesh (Variables|Default|GetStaticMesh))
  (bind _materials (Variables|Default|GetMaterials))
  (Variables|General|SetMaterial (Math|Integer|Clamp(Integer) (Variables|General|GetMaterial) 1 (Utilities|Array|Length _materials)))
  (Rendering|Material|SetMaterial (Variables|Default|GetStaticMesh) 0 (Utilities|Array|Get(acopy) _materials (- (Math|Integer|Clamp(Integer) (Variables|General|GetMaterial) 1 (Utilities|Array|Length _materials)) 1)))
  (Class|PrimitiveComponent|SetAngularDamping _staticmesh (Variables|General|GetAngular%20Damping))
  (Class|PrimitiveComponent|SetLinearDamping _staticmesh (Variables|General|GetLinear%20Damping)))