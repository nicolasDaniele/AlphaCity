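; B_Buoy is a buoy actor whose static mesh can simulate physics and float through a Buoyancy component.
; The construction script and BeginPlay both apply the exposed physics toggle and linear and angular damping to the mesh.
; The construction script destroys the Buoyancy component when buoyancy is off.
; If buoyancy is enabled without physics simulation, it prints a warning, switches buoyancy off and removes the component.
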(event EventBeginPlay
  (bind _staticmesh (Variables|Default|GetStaticMesh))
  (Physics|SetSimulatePhysics _staticmesh (Variables|General|GetSimulate%20Physics))
  (Class|PrimitiveComponent|SetAngularDamping _staticmesh (Variables|General|GetAngular%20Damping))
  (Class|PrimitiveComponent|SetLinearDamping _staticmesh (Variables|General|GetLinear%20Damping)))

(event Collision|EventActorBeginOverlap
  (params (OtherActor :type Actor%20Object%20Reference)))

(event EventTick
  (params (DeltaSeconds :type Float%20%28single-precision%29)))

(fn ConstructionScript
  (bind _staticmesh (Variables|Default|GetStaticMesh))
  (Physics|SetSimulatePhysics _staticmesh (Variables|General|GetSimulate%20Physics))
  (Class|PrimitiveComponent|SetAngularDamping _staticmesh (Variables|General|GetAngular%20Damping))
  (Class|PrimitiveComponent|SetLinearDamping _staticmesh (Variables|General|GetLinear%20Damping))
  (if (Variables|General|GetEnable%20Buoyancy)
    (if (not (Variables|General|GetSimulate%20Physics))
      (Development|PrintString "It can't have \"Enable Buoyancy\"  when \"Simulate Physics is disabled.")
      (Variables|General|SetEnable%20Buoyancy false)
      (Components|DestroyComponent (Variables|Default|GetBuoyancy) :!label _label))
    (else
      (goto _label))))