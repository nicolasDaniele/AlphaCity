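; B_Ball is a configurable beach ball prop with optional physics and buoyancy.
; The construction script picks the ball or volleyball mesh from Type, then applies the physics simulation and damping settings, which BeginPlay reapplies.
; When buoyancy is enabled, the construction script adds a buoyancy component per Type, but only with physics simulation on; otherwise it prints a warning and clears the buoyancy flag.
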(event EventBeginPlay
  (bind _staticmesh (Variables|Default|GetStaticMesh))
  (Physics|SetSimulatePhysics _staticmesh (Variables|General|GetSimulate%20Physics))
  (Class|PrimitiveComponent|SetAngularDamping _staticmesh (Variables|General|GetAngular%20Damping))
  (Class|PrimitiveComponent|SetLinearDamping _staticmesh (Variables|General|GetLinear%20Damping)))

(event Collision|EventActorBeginOverlap
  (params (OtherActor :type Actor%20Object%20Reference)))

(event EventTick
  (params (DeltaSeconds :type Float%20%28single-precision%29)))

(fn ConstructionScript
  (bind _self self)
  (bind _staticmesh (Variables|Default|GetStaticMesh))
  (switch int (Variables|General|GetType)
    (:Default
      (Components|StaticMesh|SetStaticMesh _staticmesh "/Game/BeachPack/Models/SM_VolleyBall.SM_VolleyBall" :!label _label))
    (:1
      (Components|StaticMesh|SetStaticMesh _staticmesh "/Game/BeachPack/Models/SM_Ball.SM_Ball"))
    (:2
      (goto _label)))
  (Physics|SetSimulatePhysics _staticmesh (Variables|General|GetSimulate%20Physics))
  (Class|PrimitiveComponent|SetAngularDamping _staticmesh (Variables|General|GetAngular%20Damping))
  (Class|PrimitiveComponent|SetLinearDamping _staticmesh (Variables|General|GetLinear%20Damping))
  (if (Variables|General|GetEnable%20Buoyancy)
    (if (Variables|General|GetSimulate%20Physics)
      (switch int (Variables|General|GetType)
        (:Default
          (AddComponent|AddBuoyancyComponent _self :!label _label_2))
        (:1
          (AddComponent|AddBuoyancyComponent _self))
        (:2
          (goto _label_2)))
      (else
        (Development|PrintString "It can't have \"Enable Buoyancy\"  when \"Simulate Physics is disabled.")
        (Variables|General|SetEnable%20Buoyancy false)))))