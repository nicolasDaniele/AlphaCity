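; B_Umbrella is a beach umbrella prop that builds itself in the construction script, with no active runtime logic.
; The Cloth flag chooses between adding a skeletal mesh component and a static mesh component.
; MaterialVariation is clamped to the matching material array and used as a 1-based index to set the material on the UmbrellaCloth slot.
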(event EventBeginPlay)

(event Collision|EventActorBeginOverlap
  (params (OtherActor :type Actor%20Object%20Reference)))

(event EventTick
  (params (DeltaSeconds :type Float%20%28single-precision%29)))

(fn ConstructionScript
  (Variables|General|SetMaterial%20Variation (Math|Integer|SelectInt (Math|Integer|Clamp(Integer) (Variables|General|GetMaterial%20Variation) 1 (Utilities|Array|Length (Variables|General|GetClothMaterials))) (Math|Integer|Clamp(Integer) (Variables|General|GetMaterial%20Variation) 1 (Utilities|Array|Length (Variables|General|GetMaterials))) (Variables|General|GetCloth)))
  (if (Variables|General|GetCloth)
    ;[1 0.4511 0.969] Cloth
    (bind _returnvalue (AddComponent|AddSkeletalMeshComponent false))
    (Rendering|Material|SetMaterialbyName _returnvalue "UmbrellaCloth" (Utilities|Array|Get(acopy) (Variables|General|GetClothMaterials) (- (Variables|General|GetMaterial%20Variation) 1)))
    (else
      ;[0.01465 0.7791 1] StaticMesh
      (bind _returnvalue_2 (AddComponent|AddStaticMeshComponent false))
      (Rendering|Material|SetMaterialbyName _returnvalue_2 "UmbrellaCloth" (Utilities|Array|Get(acopy) (Variables|General|GetMaterials) (- (Variables|General|GetMaterial%20Variation) 1))))))