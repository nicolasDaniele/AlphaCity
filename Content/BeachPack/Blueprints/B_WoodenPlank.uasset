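; Construction-script tool that lays a row of wooden plank meshes along a spline, for paths or walkways.
; A one-shot snap toggle line-traces spline points down onto the ground and adjusts the actor's height.
; A one-shot Randomize toggle fills editable per-plank arrays for mesh type, flips, offsets and width.
; The spawn loop applies these arrays, orienting planks to the spline and spacing them by mesh bounds plus a gap.
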(event EventBeginPlay)

(event Collision|EventActorBeginOverlap
  (params (OtherActor :type Actor%20Object%20Reference)))

(event EventTick
  (params (DeltaSeconds :type Float%20%28single-precision%29)))

(fn ConstructionScript
  (bind _distanceplanks (Variables|General|GetDistancePlanks))
  (bind _spline (Variables|Default|GetSpline))
  (bind _spline_2 (Variables|Default|GetSpline))
  (bind _defaultsceneroot (Variables|Default|GetDefaultSceneRoot))
  (bind _defaultsceneroot_2 (Variables|Default|GetDefaultSceneRoot))
  (bind _rand_x_plank_offset_ (Variables|Random|GetRand%20X%20Plank%20Offset%20))
  (bind _spline_3 (Variables|Default|GetSpline))
  (bind _rand_x_size (Variables|Random|GetRand%20X%20Size))
  (bind _spline_4 (Variables|Default|GetSpline))
  (bind _returnvalue (Spline|GetSplineLength _spline_3))
  (bind _returnvalue_2 (Spline|GetLocationatSplinePoint _spline_2 0 "World"))
  (bind _returnvalue_3 (Transformation|GetWorldLocation _defaultsceneroot_2))
  (bind (_x _y _z) (Math|Vector|BreakVector _returnvalue_3))
  (bind _returnvalue_4 (/ _returnvalue _distanceplanks))
  (bind _returnvalue_5 (Math|Float|Truncate _returnvalue_4))
  (bind _returnvalue_6 (+ _returnvalue_5 1))
  ;[0.6875 0 1] SnappingSplineToGround
  (if (Variables|Snap|GetSnappingSplineToTheGround)
    (for _index (range 0 (- (Spline|GetNumberOfSplinePoints (Variables|Default|GetSpline)) 1))
      (bind (_outhit _returnvalue_7) (Collision|LineTraceByChannel (Spline|GetLocationatSplinePoint (Variables|Default|GetSpline) _index "World") (+ (Spline|GetLocationatSplinePoint (Variables|Default|GetSpline) _index "World") "0.000000,-0.000000,-10000.000000") "TraceTypeQuery1" false 0 "None"))
      (if _returnvalue_7
        (Variables|Snap|SetLocationPoint (+ (Math|Transform|InverseTransformLocation (Math|Transform|MakeTransform (Transformation|GetWorldLocation _defaultsceneroot) (Variables|/Script/Engine.SceneComponent|GetRelativeRotation _defaultsceneroot) (Variables|/Script/Engine.SceneComponent|GetRelativeScale3D _defaultsceneroot)) (.Location (Collision|BreakHitResult _outhit))) "0, 0,2.000000"))
        (else
          (Variables|Snap|SetLocationPoint (Math|Vector|MakeVector (.X (Math|Vector|BreakVector (Spline|GetLocationatSplinePoint (Variables|Default|GetSpline) _index "Local"))) (.Y (Math|Vector|BreakVector (Spline|GetLocationatSplinePoint (Variables|Default|GetSpline) _index "Local"))) 0.0))))
      (Spline|SetLocationatSplinePoint (Variables|Default|GetSpline) _index (Variables|Snap|GetLocationPoint) "Local" true))
    (Variables|Snap|SetSnappingSplineToTheGround false)
    (Variables|Snap|SetZdifference (.Z (Math|Vector|BreakVector (- (Transformation|GetWorldLocation (Variables|Default|GetDefaultSceneRoot)) (Spline|GetLocationatSplinePoint (Variables|Default|GetSpline) 0 "World")))))
    (for _index_2 (range 0 (- (Spline|GetNumberOfSplinePoints (Variables|Default|GetSpline)) 1))
      (Spline|SetLocationatSplinePoint _spline _index_2 (+ (Spline|GetLocationatSplinePoint _spline _index_2 "Local") (Math|Vector|MakeVector 0.0 0.0 (Variables|Snap|GetZdifference))) "Local" true))
    (bind _outhit_2 (Collision|LineTraceByChannel _returnvalue_2 (+ _returnvalue_2 "0.000000,-0.000000,-10000.000000") "TraceTypeQuery1" false 0 "None"))
    (Transformation|SetWorldLocation (Variables|Default|GetDefaultSceneRoot) (+ (Math|Vector|MakeVector _x _y (- _z (- (- (.Z (Math|Vector|BreakVector _returnvalue_2)) (Variables|Snap|GetSnapOffset)) (.Z (Math|Vector|BreakVector (.Location (Collision|BreakHitResult _outhit_2))))))) "0, 0,5.000000") false false))
  ;[1 0.5445 0.3833] Resize
  (Utilities|Array|Resize (Variables|General|GetX_Planks_Offset) _returnvalue_6)
  (Utilities|Array|Resize (Variables|General|GetY_Flipped_Planks) _returnvalue_6)
  (Utilities|Array|Resize (Variables|General|GetX_Flipped_Planks) _returnvalue_6)
  (Utilities|Array|Resize (Variables|General|GetType) _returnvalue_6)
  (Utilities|Array|Resize (Variables|General|GetY_Planks_Offset) _returnvalue_6)
  (Utilities|Array|Resize (Variables|General|GetX_Planks_Scale) _returnvalue_6)
  ;[0.2923 0.4974 1] Type Clamp
  (for (_array_element _array_index) (Variables|General|GetType)
    (Utilities|Array|SetArrayElem (Variables|General|GetType) _array_index (Math|Integer|Clamp(Integer) _array_element 1 (Utilities|Array|Length (Variables|Default|GetStaticMeshes)))))
  ;[1 0.269 0.3188] Random
  (if (Variables|Random|GetRandomize)
    (for (_ _array_index_2) (Variables|General|GetX_Planks_Offset)
      (Utilities|Array|SetArrayElem (Variables|General|GetX_Planks_Offset) _array_index_2 (Math|Random|RandomFloatinRange (* _rand_x_plank_offset_ -1.0) _rand_x_plank_offset_)))
    (for (_ _array_index_3) (Variables|General|GetY_Flipped_Planks)
      (Utilities|Array|SetArrayElem (Variables|General|GetY_Flipped_Planks) _array_index_3 (Math|Random|RandomBool)))
    (for (_ _array_index_4) (Variables|General|GetX_Flipped_Planks)
      (Utilities|Array|SetArrayElem (Variables|General|GetX_Flipped_Planks) _array_index_4 (Math|Random|RandomBool)))
    (for (_ _array_index_5) (Variables|General|GetType)
      (Utilities|Array|SetArrayElem (Variables|General|GetType) _array_index_5 (Math|Random|RandomIntegerinRange 1 (Utilities|Array|Length (Variables|Default|GetStaticMeshes)))))
    (for (_ _array_index_6) (Variables|General|GetY_Planks_Offset)
      (Utilities|Array|SetArrayElem (Variables|General|GetY_Planks_Offset) _array_index_6 (Math|Random|RandomFloatinRange 0.0 (Variables|Random|GetRand%20Y%20Plank%20Offset%20))))
    (for (_ _array_index_7) (Variables|General|GetX_Planks_Scale)
      (Utilities|Array|SetArrayElem (Variables|General|GetX_Planks_Scale) _array_index_7 (Math|Random|RandomFloatinRange (* _rand_x_size -1.0) _rand_x_size)))
    (Variables|Random|SetRandomize false))
  (Variables|Temp|SetTempInt -1)
  (while (< (Variables|Temp|GetCurrentDistance) (Spline|GetSplineLength (Variables|Default|GetSpline)))
    (Math|Integer|IncrementInt (Variables|Temp|GetTempInt)
      (:%20%20
        (bind _returnvalue_8 (AddComponent|AddStaticMeshComponent false))
        (Components|StaticMesh|SetStaticMesh _returnvalue_8 (Utilities|Array|Get(acopy) (Variables|Default|GetStaticMeshes) (- (Utilities|Array|Get(acopy) (Variables|General|GetType) (Variables|Temp|GetTempInt)) 1)))
        (Transformation|SetRelativeScale3D _returnvalue_8 (* (Math|Vector|MakeVector 1.0 (Math|Float|SelectFloat -1.0 1.0 (Utilities|Array|Get(acopy) (Variables|General|GetX_Flipped_Planks) (Variables|Temp|GetTempInt))) (Math|Float|SelectFloat -1.0 1.0 (Utilities|Array|Get(acopy) (Variables|General|GetY_Flipped_Planks) (Variables|Temp|GetTempInt)))) (Math|Vector|MakeVector 1.0 (+ 1.0 (/ (Variables|General|GetScale%20X) 1e+01) (/ (Utilities|Array|Get(acopy) (Variables|General|GetX_Planks_Scale) (Variables|Temp|GetTempInt)) 1e+01)) (+ 1.0 (/ (Variables|General|GetScale%20Y) 1e+01)))))
        ;[1 0.6039 0.5239] Rotation
        (Transformation|SetRelativeRotation _returnvalue_8 (Spline|GetRotationatDistanceAlongSpline (Variables|Default|GetSpline) (Variables|Temp|GetCurrentDistance) "Local") false false)
        ;[1 0.807 0.256] Location
        (Transformation|SetRelativeLocation _returnvalue_8 (+ (Math|Vector|MakeVector 0.0 0.0 (Utilities|Array|Get(acopy) (Variables|General|GetY_Planks_Offset) (Variables|Temp|GetTempInt))) (+ (* (Class|SplineComponent|GetRightVectoratDistanceAlongSpline _spline_4 (Variables|Temp|GetCurrentDistance) "Local") (Math|Vector|MakeVector (Utilities|Array|Get(acopy) (Variables|General|GetX_Planks_Offset) (Variables|Temp|GetTempInt)) (Utilities|Array|Get(acopy) (Variables|General|GetX_Planks_Offset) (Variables|Temp|GetTempInt)) (Utilities|Array|Get(acopy) (Variables|General|GetX_Planks_Offset) (Variables|Temp|GetTempInt)))) (Spline|GetLocationatDistanceAlongSpline _spline_4 (Variables|Temp|GetCurrentDistance) "Local"))) false false)
        (Variables|Temp|SetCurrentDistance (+ (Variables|Temp|GetCurrentDistance) (+ (Variables|General|GetDistancePlanks) (* (.X (Math|Vector|BreakVector (.max (StaticMesh|GetBoundingBox (Variables|/Script/Engine.StaticMeshComponent|GetStaticMesh _returnvalue_8))))) 2.0))))))))